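; Base Blueprint for interactable objects that show a text prompt while something overlaps their interaction radius.
; Interact shows locked text if locked; otherwise it hides the radius and prompt, then calls StartEventOnInteract, an empty hook for child classes to override.
; Unlock clears the lock and swaps in the unlocked text.
; An InteractComplete flag suppresses interaction and prompt toggling, though this parent never sets it.
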(event OnComponentBeginOverlap(InteractionRadius)
  (params (OverlappedComponent :type Primitive%20Component%20Object%20Reference) (OtherActor :type Actor%20Object%20Reference) (OtherComp :type Primitive%20Component%20Object%20Reference) (OtherBodyIndex :type Integer) (bFromSweep :type Boolean) (SweepResult :type Hit%20Result%20Structure%20%28by%20ref%29))
  (if (not (Variables|Default|GetInteractComplete))
    (Development|SetHiddeninGame (Variables|Default|GetTextRender) false false)))

(event OnComponentEndOverlap(InteractionRadius)
  (params (OverlappedComponent :type Primitive%20Component%20Object%20Reference) (OtherActor :type Actor%20Object%20Reference) (OtherComp :type Primitive%20Component%20Object%20Reference) (OtherBodyIndex :type Integer))
  (if (not (Variables|Default|GetInteractComplete))
    (Development|SetHiddeninGame (Variables|Default|GetTextRender) true false)))

(event Custom|StartEventOnInteract)

(event EventUnlock
  (Variables|Default|SetIsLocked false)
  (Rendering|Components|TextRender|SetText (Variables|Default|GetTextRender) (Variables|Default|GetUnlockedText)))

(event EventInteract
  (if (not (Variables|Default|GetInteractComplete))
    (if (Variables|Default|GetIsLocked)
      (Rendering|Components|TextRender|SetText (Variables|Default|GetTextRender) (Variables|Default|GetLockedText))
      (else
        (Development|SetHiddeninGame (Variables|Default|GetInteractionRadius) true false)
        (Development|SetHiddeninGame (Variables|Default|GetTextRender) true false)
        (CallFunction|StartEventonInteract)))))

(fn ConstructionScript)