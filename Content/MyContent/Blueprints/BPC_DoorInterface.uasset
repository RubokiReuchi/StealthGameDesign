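; Door Blueprint, derived from a parent class, that responds to Interact and Unlock events and can be locked.
; Interact shows the locked text on a TextRender while IsLocked is set, and otherwise calls InteractWithDoor.
; Unlock clears IsLocked and switches the TextRender to the unlocked text.
; The construction script only runs the parent's version.
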(event EventUnlock
  (Variables|Default|SetIsLocked false)
  (Rendering|Components|TextRender|SetText (Variables|Default|GetTextRender) (Variables|Default|GetUnlockedText)))

(event EventInteract
  (if (Variables|Default|GetIsLocked)
    (Rendering|Components|TextRender|SetText (Variables|Default|GetTextRender) (Variables|Default|GetLockedText))
    (else
      (CallFunction|InteractwithDoor))))

(fn ConstructionScript
  (|CallParentFunction))