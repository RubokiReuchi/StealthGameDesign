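; Interactable switch that can start locked and, when used, presses down once and signals that the interaction is complete.
; The interact event passes a DoOnce into a timeline that lowers the mesh, then sets the completion flag and fires the completion dispatcher.
; The construction script colors the mesh red or green from the lock state; Unlock clears the lock, updates the text and turns it green.
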(event EventUnlock
  (Variables|Default|SetIsLocked false)
  (Rendering|Components|TextRender|SetText (Variables|Default|GetTextRender) (Variables|Default|GetUnlockedText))
  (Rendering|Material|SetMaterial (Variables|Default|GetStaticMesh) 0 "/Game/Materials/MI_LDGrid_Green.MI_LDGrid_Green"))

(event EventStartEventonInteract
  (Utilities|FlowControl|DoOnce false
    (:Completed
      (bind _newtrack_0 (Timeline|Timeline Play)
        (:Update
          (Transformation|SetRelativeLocation (Variables|Default|GetStaticMesh) (Math|Vector|Lerp(Vector) "0, 0, 0" "0.000000,0.000000,-10.000000" _newtrack_0) false false))
        (:Finished
          (Variables|Default|SetInteractComplete true)
          (Default|CallOnInteractionComplete))))))

(fn ConstructionScript
  (bind _staticmesh (Variables|Default|GetStaticMesh))
  (|CallParentFunction)
  (if (Variables|Default|GetIsLocked)
    (Rendering|Material|SetMaterial _staticmesh 0 "/Game/Materials/MI_LDGrid_Red.MI_LDGrid_Red")
    (else
      (Rendering|Material|SetMaterial _staticmesh 0 "/Game/Materials/MI_LDGrid_Green.MI_LDGrid_Green"))))