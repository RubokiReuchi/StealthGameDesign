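; Barricade interactable, built on a parent interaction class, that collapses when the player interacts with it.
; On interaction start, its five static meshes switch to physics simulation and are woken so they can fall.
; After a short delay the meshes are hidden, not destroyed, and the interaction is flagged complete and signalled through the completion call.
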(event EventStartEventonInteract
  (bind _staticmesh4 (Variables|Default|GetStaticMesh4))
  (Physics|SetSimulatePhysics (Variables|Default|GetStaticMesh3) true)
  (Class|PrimitiveComponent|WakeAllRigidBodies _staticmesh4)
  (Utilities|FlowControl|Delay 2.0)
  (Development|SetHiddeninGame _staticmesh4 true false)
  (Variables|Default|SetInteractComplete true)
  (Default|CallOnInteractionComplete))

(fn ConstructionScript
  (|CallParentFunction))