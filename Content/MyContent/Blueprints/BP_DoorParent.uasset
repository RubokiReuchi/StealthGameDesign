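; BP_DoorParent is an interactable door, named as a parent Blueprint, that swings open and closed around yaw.
; Its InteractWithDoor event plays or reverses the DoorAnimation timeline based on IsOpen, lerping the Door's relative rotation.
; When the timeline finishes, it flips IsOpen and toggles the TextRender's visibility.
; Overlapping the InteractiveRadius component shows the text in game, and leaving hides it.
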(event OnComponentBeginOverlap(InteractiveRadius)
  (params (OverlappedComponent :type Primitive%20Component%20Object%20Reference) (OtherActor :type Actor%20Object%20Reference) (OtherComp :type Primitive%20Component%20Object%20Reference) (OtherBodyIndex :type Integer) (bFromSweep :type Boolean) (SweepResult :type Hit%20Result%20Structure%20%28by%20ref%29))
  ;[1 1 1] Enter/Exit Door
  (Development|SetHiddeninGame (Variables|Default|GetTextRender) false false))

(event OnComponentEndOverlap(InteractiveRadius)
  (params (OverlappedComponent :type Primitive%20Component%20Object%20Reference) (OtherActor :type Actor%20Object%20Reference) (OtherComp :type Primitive%20Component%20Object%20Reference) (OtherBodyIndex :type Integer))
  ;[1 1 1] Enter/Exit Door
  (Development|SetHiddeninGame (Variables|Default|GetTextRender) true false))

(event Custom|InteractWithDoor
  ;[1 1 1] Animation
  (if (Variables|Default|GetIsOpen)
    (bind _dooralpha (Timeline|DoorAnimation Reverse)
      (:Update
        (Transformation|SetRelativeRotation (Variables|Default|GetDoor) (Math|Rotator|Lerp(Rotator) "0, 0, 0" "0.000000,110.000000,0.000000" _dooralpha) false false))
      (:Finished
        (Variables|Default|SetIsOpen (not (Variables|Default|GetIsOpen)))
        (Rendering|ToggleVisibility (Variables|Default|GetTextRender) false)))
    (else
      (Timeline|DoorAnimation Play))))

(fn ConstructionScript)