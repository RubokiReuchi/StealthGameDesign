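; Interactable ladder that the player first places, then uses to jump between its two ends.
; When unlocked, the first interaction reveals the mesh and prompt and switches both text renders to the use-ladder text.
; Later interactions move the ALS character, found by class lookup, instantly to the opposite interaction radius, with no climbing.
; Radius overlaps set the Bottom flag that picks the destination; the second radius also toggles its prompt.
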(event OnComponentBeginOverlap(InteractionRadius1)
  (params (OverlappedComponent :type Primitive%20Component%20Object%20Reference) (OtherActor :type Actor%20Object%20Reference) (OtherComp :type Primitive%20Component%20Object%20Reference) (OtherBodyIndex :type Integer) (bFromSweep :type Boolean) (SweepResult :type Hit%20Result%20Structure%20%28by%20ref%29))
  (Variables|Default|SetBottom true)
  (Development|SetHiddeninGame (Variables|Default|GetTextRender1) false false))

(event OnComponentBeginOverlap(InteractionRadius)
  (params (OverlappedComponent :type Primitive%20Component%20Object%20Reference) (OtherActor :type Actor%20Object%20Reference) (OtherComp :type Primitive%20Component%20Object%20Reference) (OtherBodyIndex :type Integer) (bFromSweep :type Boolean) (SweepResult :type Hit%20Result%20Structure%20%28by%20ref%29))
  (Variables|Default|SetBottom false))

(event OnComponentEndOverlap(InteractionRadius1)
  (params (OverlappedComponent :type Primitive%20Component%20Object%20Reference) (OtherActor :type Actor%20Object%20Reference) (OtherComp :type Primitive%20Component%20Object%20Reference) (OtherBodyIndex :type Integer))
  (Development|SetHiddeninGame (Variables|Default|GetTextRender1) true false))

(event EventStartEventonInteract
  (if (not (Variables|Default|GetIsLocked))
    (if (Variables|Default|GetPlaced)
      (bind _returnvalue (Actor|GetActorOfClass "/Game/AdvancedLocomotionV4/Blueprints/CharacterLogic/ALS_AnimMan_CharacterBP.ALS_AnimMan_CharacterBP_C"))
      (if (Variables|Default|GetBottom)
        (Transformation|SetActorLocation _returnvalue (Transformation|GetWorldLocation (Variables|Default|GetInteractionRadius)) false false)
        (else
          (Transformation|SetActorLocation _returnvalue (Transformation|GetWorldLocation (Variables|Default|GetInteractionRadius1)) false false)))
      (else
        (Development|SetHiddeninGame (Variables|Default|GetStaticMesh) false false)
        (Development|SetHiddeninGame (Variables|Default|GetTextRender) false false)
        (Variables|Default|SetPlaced true)
        (Rendering|Components|TextRender|SetText (Variables|Default|GetTextRender) (Variables|Default|GetUseLadderText))))))

(fn ConstructionScript
  (|CallParentFunction))