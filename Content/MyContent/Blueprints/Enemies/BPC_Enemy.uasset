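; Patrolling stealth enemy that follows a spline via timeline and respawns the player on sight.
; PauseMovement halts it for a delay, optionally sweeping the head.
; Cone overlaps enable Tick, which line-traces from head to player, ignoring other enemies, and reddens the spotlight on detection; Energize switches from small to big cone and light.
; Interact disables and hides the enemy, rolling a key drop whose chance rises after each failure.
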(event OnComponentBeginOverlap(BigCone)
  (params (OverlappedComponent :type Primitive%20Component%20Object%20Reference) (OtherActor :type Actor%20Object%20Reference) (OtherComp :type Primitive%20Component%20Object%20Reference) (OtherBodyIndex :type Integer) (bFromSweep :type Boolean) (SweepResult :type Hit%20Result%20Structure%20%28by%20ref%29))
  ;[1 1 1] Player detection
  (if (Variables|Default|GetLightsOn)
    (bind _asals_anim_man_character_bp (Utilities|Casting|CastToALS_AnimMan_CharacterBP OtherActor))
    (Variables|Default|SetPlayerReference _asals_anim_man_character_bp)
    (Actor|Tick|SetActorTickEnabled true)))

(event OnComponentEndOverlap(BigCone)
  (params (OverlappedComponent :type Primitive%20Component%20Object%20Reference) (OtherActor :type Actor%20Object%20Reference) (OtherComp :type Primitive%20Component%20Object%20Reference) (OtherBodyIndex :type Integer))
  ;[1 1 1] Player detection
  (if (Variables|Default|GetLightsOn)
    (Utilities|Casting|CastToALS_AnimMan_CharacterBP OtherActor)
    (Rendering|Components|Light|SetLightColor (Variables|Default|GetBigSpotLight) "(R=1.000000,G=1.000000,B=1.000000,A=1.000000)" true)
    (Actor|Tick|SetActorTickEnabled false)))

(event OnComponentBeginOverlap(SmallCone)
  (params (OverlappedComponent :type Primitive%20Component%20Object%20Reference) (OtherActor :type Actor%20Object%20Reference) (OtherComp :type Primitive%20Component%20Object%20Reference) (OtherBodyIndex :type Integer) (bFromSweep :type Boolean) (SweepResult :type Hit%20Result%20Structure%20%28by%20ref%29))
  ;[1 1 1] Player detection
  (if (not (Variables|Default|GetLightsOn))
    (bind _asals_anim_man_character_bp (Utilities|Casting|CastToALS_AnimMan_CharacterBP OtherActor))
    (Variables|Default|SetPlayerReference _asals_anim_man_character_bp)
    (Actor|Tick|SetActorTickEnabled true)))

(event OnComponentEndOverlap(SmallCone)
  (params (OverlappedComponent :type Primitive%20Component%20Object%20Reference) (OtherActor :type Actor%20Object%20Reference) (OtherComp :type Primitive%20Component%20Object%20Reference) (OtherBodyIndex :type Integer))
  ;[1 1 1] Player detection
  (if (not (Variables|Default|GetLightsOn))
    (Utilities|Casting|CastToALS_AnimMan_CharacterBP OtherActor)
    (Rendering|Components|Light|SetLightColor (Variables|Default|GetSmallSpotLight) "(R=1.000000,G=1.000000,B=1.000000,A=1.000000)" true)
    (Actor|Tick|SetActorTickEnabled false)))

(event Custom|Move%20Enemy
  (bind _pathspline (Variables|Default|GetPathSpline))
  (bind _spline (Variables|/Game/MyContent/Blueprints/Enemies/BP_Spline.BP_Spline_C|GetSpline _pathspline))
  (Components|Timeline|SetPlayRate (Variables|Default|GetTimeline) (/ 1.0 (Variables|Default|GetSecondsToCompletePathLoop)))
  (bind _track (Timeline|Timeline Play)
    (:Update
      (Transformation|SetActorTransform (Math|Transform|MakeTransform (Spline|GetLocationatDistanceAlongSpline _spline (Math|Float|Lerp 0.0 (Spline|GetSplineLength _spline) _track) "World") (Math|Rotator|MakeRotator 0.0 0.0 (.yaw (Spline|GetRotationatDistanceAlongSpline _spline (Math|Float|Lerp 0.0 (Spline|GetSplineLength _spline) _track) "World"))) "1.000000,1.000000,1.000000")))))

(event Custom|PauseMovement
  (params (Delay :type Float%20%28double-precision%29))
  (Audio|Components|Audio|Stop (Variables|Default|GetTimeline))
  (if (Variables|Default|GetRotateHeadBool)
    (Components|Timeline|SetPlayRate (Variables|Default|GetRotateHead) (/ 1.0 Delay))
    (bind _angle (Timeline|RotateHead PlayFromStart)
      (:Update
        (Transformation|SetRelativeRotation (Variables|Default|GetHeaD) (Math|Rotator|Lerp(Rotator) "0.000000,-90.000000,0.000000" "0.000000,90.000000,0.000000" _angle) false false))
      (:Finished
        (Audio|Components|Audio|Play (Variables|Default|GetTimeline) :!label _label)))
    (else
      (Utilities|FlowControl|Delay Delay)
      (goto _label))))

(event EventBeginPlay
  (bind _outactors (Actor|GetAllActorsOfClass "BPC_Enemy_C"))
  (Variables|Default|SetOtherEnemies _outactors)
  (Utilities|IsValid (Variables|Default|GetPathSpline)
    (:Is%20Valid
      (CallFunction|MoveEnemy))))

(event EventEnergize
  ;[1 1 1] Player detection
  (Development|SetHiddeninGame (Variables|Default|GetSmallSpotLight) true false)
  (Development|SetHiddeninGame (Variables|Default|GetSmallCone) true false)
  (Development|SetHiddeninGame (Variables|Default|GetBigSpotLight) false false)
  (Development|SetHiddeninGame (Variables|Default|GetBigCone) false false)
  (Variables|Default|SetLightsOn true))

(event EventTick
  (params (DeltaSeconds :type Float%20%28single-precision%29))
  (bind _playerreference (Variables|Default|GetPlayerReference))
  (bind _outhit (Collision|LineTraceByChannel (Transformation|GetWorldLocation (Variables|Default|GetHeaD)) (Transformation|GetActorLocation _playerreference) "TraceTypeQuery1" false (Variables|Default|GetOtherEnemies) "None"))
  (if (== (.HitActor (Collision|BreakHitResult _outhit)) _playerreference)
    (if (Variables|Default|GetLightsOn)
      (Rendering|Components|Light|SetLightColor (Variables|Default|GetBigSpotLight) "(R=1.000000,G=0.000000,B=0.000000,A=1.000000)" true)
      (else
        (Rendering|Components|Light|SetLightColor (Variables|Default|GetSmallSpotLight) "(R=1.000000,G=0.000000,B=0.000000,A=1.000000)" true)))
    (Default|Respawn _playerreference)))

(event EventInteract
  (bind _enemykey (Variables|Default|GetEnemyKey))
  (bind _enemykey_2 (Variables|Default|GetEnemyKey))
  (Collision|SetActorEnableCollision false)
  (Rendering|SetActorHiddenInGame true)
  (Utilities|IsValid _enemykey
    (:Is%20Valid
      (if (not (Variables|/Game/MyContent/Blueprints/BPC_EnemyKey.BPC_EnemyKey_C|GetPicked _enemykey))
        (if (< (Math|Random|RandomFloat) (Variables|/Game/MyContent/Blueprints/BPC_EnemyKey.BPC_EnemyKey_C|GetDropChance _enemykey))
          (Transformation|SetActorLocation _enemykey_2 (+ (Transformation|GetActorLocation) "0.000000,0.000000,140.000000") false false)
          (Rendering|SetActorHiddenInGame _enemykey_2 false)
          (Variables|/Game/MyContent/Blueprints/BPC_EnemyKey.BPC_EnemyKey_C|SetPicked _enemykey_2 true)
          (else
            (Variables|/Game/MyContent/Blueprints/BPC_EnemyKey.BPC_EnemyKey_C|SetDropChance _enemykey (+ (Variables|/Game/MyContent/Blueprints/BPC_EnemyKey.BPC_EnemyKey_C|GetDropChance _enemykey) (Variables|/Game/MyContent/Blueprints/BPC_EnemyKey.BPC_EnemyKey_C|GetIncreaseDropChance _enemykey)))))))))

(fn ConstructionScript
  (|CallParentFunction))