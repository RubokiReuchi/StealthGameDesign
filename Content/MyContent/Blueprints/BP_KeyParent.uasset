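; BP_KeyParent is a base key pickup that unlocks linked actors when the player interacts with it.
; An overlap radius toggles a text prompt while the key is untaken.
; The first Interact marks it taken, hides text and mesh, disables collision, and sends UnlockMessage to each ActorsToUnlock entry implementing BPI_Interaction.
; It then calls StartEventsOnTaken, an empty hook for child Blueprints.
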(event OnComponentBeginOverlap(InteractionRadius)
  (params (OverlappedComponent :type Primitive%20Component%20Object%20Reference) (OtherActor :type Actor%20Object%20Reference) (OtherComp :type Primitive%20Component%20Object%20Reference) (OtherBodyIndex :type Integer) (bFromSweep :type Boolean) (SweepResult :type Hit%20Result%20Structure%20%28by%20ref%29))
  (if (not (Variables|Default|GetIsTaken))
    (Development|SetHiddeninGame (Variables|Default|GetTextRender) false false)))

(event OnComponentEndOverlap(InteractionRadius)
  (params (OverlappedComponent :type Primitive%20Component%20Object%20Reference) (OtherActor :type Actor%20Object%20Reference) (OtherComp :type Primitive%20Component%20Object%20Reference) (OtherBodyIndex :type Integer))
  (if (not (Variables|Default|GetIsTaken))
    (Development|SetHiddeninGame (Variables|Default|GetTextRender) true false)))

(event Custom|StartEventsOnTaken)

(event EventInteract
  (Utilities|FlowControl|DoOnce false
    (:Completed
      (Variables|Default|SetIsTaken true)
      (Development|SetHiddeninGame (Variables|Default|GetTextRender) true false)
      (Collision|SetActorEnableCollision false)
      (for _array_element (Variables|Default|GetActorsToUnlock)
        (if (Utilities|DoesObjectImplementInterface _array_element "/Game/MyContent/Interfaces/BPI_Interaction.BPI_Interaction_C")
          (Class|BPIInteraction|Unlock(Message) _array_element)))
      (CallFunction|StartEventsonTaken))))

(fn ConstructionScript)