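; Interactable gear machine that the player places, then rotates once it has energy, built as a child of a parent interactable Blueprint.
; First interaction reveals the mesh and status text; Energize supplies power and updates the label.
; Each powered interaction fires interaction complete, then a Timeline pitches the gear a quarter turn.
; After a cooldown it decrements AvailableRotations, setting InteractComplete at zero or showing the text again otherwise.
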(event EventEnergize
  (Variables|Default|SetHaveEnergy true)
  (if (not (Variables|Default|GetIsLocked))
    (if (Variables|Default|GetPlaced)
      (Rendering|Components|TextRender|SetText (Variables|Default|GetTextRender) (Variables|Default|GetEnergy)))))

(event EventStartEventonInteract
  (bind _textrender (Variables|Default|GetTextRender))
  (bind _textrender_2 (Variables|Default|GetTextRender))
  (bind _staticmesh (Variables|Default|GetStaticMesh))
  (if (Variables|Default|GetPlaced)
    (if (Variables|Default|GetHaveEnergy)
      (if (not (Variables|Default|GetRotating))
        (Variables|Default|SetRotating true)
        (Variables|Default|SetRotation (Variables|/Script/Engine.SceneComponent|GetRelativeRotation _staticmesh))
        (Default|CallOnInteractionComplete)
        (bind _progression (Timeline|Timeline PlayFromStart)
          (:Update
            (Transformation|SetRelativeRotation (Variables|Default|GetStaticMesh) (Math|Rotator|Lerp(Rotator) (Math|Rotator|MakeRotator 0.0 (.pitch (Variables|Default|GetRotation)) 9e+01) (Math|Rotator|MakeRotator 0.0 (+ (.pitch (Variables|Default|GetRotation)) 9e+01) 9e+01) _progression) false false))
          (:Finished
            (Utilities|FlowControl|Delay 3.0)
            (Variables|Default|SetRotating false)
            (Variables|Default|SetAvailableRotations (+ (Variables|Default|GetAvailableRotations) -1))
            (if (== (Variables|Default|GetAvailableRotations) 0)
              (Variables|Default|SetInteractComplete true)
              (else
                (Development|SetHiddeninGame _textrender_2 false false))))))
      (else
        (Development|SetHiddeninGame _textrender false false)
        (Rendering|Components|TextRender|SetText _textrender_2 (Variables|Default|GetNoEnergy) :!label _label)))
    (else
      (Development|SetHiddeninGame _staticmesh false false)
      (Development|SetHiddeninGame _textrender false false)
      (Variables|Default|SetIsLocked false)
      (Variables|Default|SetPlaced true)
      (if (Variables|Default|GetHaveEnergy)
        (Rendering|Components|TextRender|SetText (Variables|Default|GetTextRender) (Variables|Default|GetEnergy))
        (else
          (goto _label))))))

(fn ConstructionScript
  (|CallParentFunction))